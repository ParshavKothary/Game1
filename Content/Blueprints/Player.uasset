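; Player paddle for a two-player puck game, which sends any Puck overlapping its Box off along the aim direction at HitSpeed.
; Player two teleports to a Player2StartBP and turns blue on BeginPlay.
; Each tick derives aim from paddle to crosshair, mirrors the angle by player and clamps it to a 120-degree cone.
; That angle rotates the Arrow and offsets it around the paddle using trigonometry.
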(event `self.Box.OnComponentBeginOverlap`
  (params (OverlappedComponent :type "PrimitiveComponent Object Reference") (OtherActor :type "Actor Object Reference") (OtherComp :type "PrimitiveComponent Object Reference") (OtherBodyIndex :type Integer) (bFromSweep :type Boolean) (SweepResult :type "HitResult Structure (by ref)"))
  (bind _aspuck (cast `/Game/Blueprints/Puck` OtherActor))
  (set `/Game/Blueprints/Puck.mVelocity` (* (`KismetMathLibrary.Normal` (`self.AimVector`)) (`self.HitSpeed`)) _aspuck))

(event `self.ReceiveBeginPlay`
  (if (not (`self.IsPlayerOne`))
    (bind _outactors (`GameplayStatics.GetAllActorsOfClass` "/Game/Blueprints/Player2StartBP.Player2StartBP_C"))
    (for _array_element _outactors
      (`self.K2_SetActorTransform` (`self.GetTransform` _array_element) false true)
      (break))
    (`PrimitiveComponent.SetMaterial` (`self.Cube`) 0 "/Game/Materials/PaddleBlue.PaddleBlue")
    (`PrimitiveComponent.SetMaterial` (`self.Crosshair`) 0 "/Game/Materials/PaddleBlue.PaddleBlue")))

(event `self.ReceiveTick`
  (params (DeltaSeconds :type "Float (single-precision)"))
  (`self.SetArrowRotation`)
  (`self.SetArrowOffset`)
  (`SceneComponent.SetVisibility` (`self.Widget`) true false))

(fn `AngleBetweenVectors`
  (params (A :type "Vector Structure") (B :type "Vector Structure"))
  (returns (Angle :type "Float (double-precision)"))
  (bind _returnvalue (`KismetMathLibrary.Normal` A))
  (bind _returnvalue_2 (`KismetMathLibrary.Normal` B))
  (bind _isplayerone (`self.IsPlayerOne`))
  (bind _returnvalue_3 (`KismetMathLibrary.DegAcos` (`KismetMathLibrary.Dot_VectorVector` _returnvalue _returnvalue_2)))
  (if (< (.x _returnvalue) (.x _returnvalue_2))
    (if _isplayerone
      _
      (else
        (return _returnvalue_3)))
    (elif _isplayerone
      (return _returnvalue_3)
      (else
        _)))
  (return (- 360.0 _returnvalue_3)))

(fn `SetArrowOffset`
  (bind _aimangle (`self.AimAngle`))
  (set `self.ArrowOffsetX` (* (`KismetMathLibrary.DegSin` (- 360.0 _aimangle)) 33.0))
  (set `self.ArrowOffsetY` (- 200.0 (- 82.0 (* (`KismetMathLibrary.DegCos` _aimangle) 50.0))))
  (`SceneComponent.K2_SetRelativeLocation` (`self.Arrow`) (`KismetMathLibrary.MakeVector` (`self.ArrowOffsetX`) (`self.ArrowOffsetY`)) false true)
  (return))

(fn `SetArrowRotation`
  (bind _cube (`self.Cube`))
  (bind _output_get (set `self.AimVector` (- (`KismetMathLibrary.MakeVector` (.x (`SceneComponent.K2_GetComponentLocation` (`self.Crosshair`))) (.y (`SceneComponent.K2_GetComponentLocation` (`self.Crosshair`)))) (`KismetMathLibrary.MakeVector` (.x (`SceneComponent.K2_GetComponentLocation` _cube)) (.y (`SceneComponent.K2_GetComponentLocation` _cube))))))
  (bind _angle (`self.AngleBetweenVectors` (`KismetMathLibrary.MakeVector` (.y (`SceneComponent.GetForwardVector` _cube)) (.x (`SceneComponent.GetForwardVector` _cube))) _output_get))
  (if (and (< _angle 300.0) (>= _angle 180.0))
    (set `self.AimAngle` 300.0)
    (set `self.AimVector` (1.732 1.0 0.0))
    (elif (and (>= _angle 60.0) (< _angle 180.0))
      (set `self.AimAngle` 60.0)
      (set `self.AimVector` (-1.732 1.0 0.0))
      (else
        (set `self.AimAngle` _angle))))
  (`SceneComponent.K2_SetWorldRotation` (`self.Arrow`) (`KismetMathLibrary.MakeRotator` 0.0 0.0 (`self.AimAngle`)) false false)
  (return))

(fn `UserConstructionScript`)