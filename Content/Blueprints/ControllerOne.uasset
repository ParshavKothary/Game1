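; Player controller that drives a Player pawn's movement along world X and its aiming crosshair, for player one or two.
; The controller ID sets the player role at BeginPlay, which mirrors which stick moves and which aims.
; Each tick, movement integrates stick acceleration with a speed cap and half-rate coasting deceleration, using a swept Cube offset that backs off and stops on blocking hits.
; Aiming offsets the Crosshair per frame, clamped to a rectangle.
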(event `self.ReceiveBeginPlay`
  (set `self.AbsAccel` 300.0)
  (set `self.MoveSpeed` 0.0)
  (set `self.AbsSpeedMax` 20.0)
  (set `self.AimSpeed` 15.0)
  (bind _asplayer (cast `/Game/Blueprints/Player` (`self.K2_GetPawn`))
    (:`then`
      (bind _output_get (set `self.mPlayer` _asplayer))
      (bind _returnvalue (`GameplayStatics.GetPlayerControllerID` self))
      (bind _output_get_2 (set `self.IsPlayerOne` (== _returnvalue 0)))
      (set `/Game/Blueprints/Player.IsPlayerOne` _output_get_2 _output_get))
    (:`CastFailed`
      (set `self.PawnFound` false))))

(event `self.ReceiveTick`
  (params (DeltaSeconds :type "Float (single-precision)"))
  (if (`self.PawnFound`)
    (`|ExecutionSequence`
      (:`then_0`
        (`self.ProcessMove`))
      (:`then_1`
        (`self.ProcessAim`)))))

(fn `GetAimAxisRight`
  (returns (AimAxisRight :type "Float (double-precision)"))
  (if (`self.IsPlayerOne`)
    (return (`self.GetInputAxisValue`))
    (else
      (return (`self.GetInputAxisValue`)))))

(fn `GetAimAxisUp`
  (returns (AimAxisUp :type "Float (double-precision)"))
  (if (`self.IsPlayerOne`)
    (return (`self.GetInputAxisValue`))
    (else
      (return (`self.GetInputAxisValue`)))))

(fn `GetMoveAxis`
  (returns (MoveAxis :type "Float (double-precision)"))
  (if (`self.IsPlayerOne`)
    (return (`self.GetInputAxisValue`))
    (else
      (return (`self.GetInputAxisValue`)))))

(fn `ProcessAim`
  (bind _x (.x (`self.AimLimitBottomRight`)))
  (bind _y (.y (`self.AimLimitBottomRight`)))
  (bind _x_2 (.x (`self.AimLimitTopLeft`)))
  (bind _y_2 (.y (`self.AimLimitTopLeft`)))
  (bind _crosshair (`/Game/Blueprints/Player.Crosshair` (`self.mPlayer`)))
  (bind _crosshair_2 (`/Game/Blueprints/Player.Crosshair` (`self.mPlayer`)))
  (bind _crosshair_3 (`/Game/Blueprints/Player.Crosshair` (`self.mPlayer`)))
  (bind _crosshair_4 (`/Game/Blueprints/Player.Crosshair` (`self.mPlayer`)))
  (bind _aimaxisup (`self.GetAimAxisUp`))
  (bind _aimaxisright (`self.GetAimAxisRight`))
  (`SceneComponent.K2_AddWorldOffset` _crosshair_4 (* (`KismetMathLibrary.MakeVector` _aimaxisup _aimaxisright) (`self.AimSpeed`)) false false)
  (if (> (.x (`SceneComponent.K2_GetComponentLocation` _crosshair_4)) _x_2)
    (`SceneComponent.K2_SetWorldLocation` _crosshair_4 (`KismetMathLibrary.MakeVector` _x_2 (.y (`SceneComponent.K2_GetComponentLocation` _crosshair_4)) (.z (`SceneComponent.K2_GetComponentLocation` _crosshair_4))) false false))
  (if (< (.y (`SceneComponent.K2_GetComponentLocation` _crosshair_2)) _y_2)
    (`SceneComponent.K2_SetWorldLocation` _crosshair_2 (`KismetMathLibrary.MakeVector` (.x (`SceneComponent.K2_GetComponentLocation` _crosshair_2)) _y_2 (.z (`SceneComponent.K2_GetComponentLocation` _crosshair_2))) false false))
  (if (< (.x (`SceneComponent.K2_GetComponentLocation` _crosshair)) _x)
    (`SceneComponent.K2_SetWorldLocation` _crosshair (`KismetMathLibrary.MakeVector` _x (.y (`SceneComponent.K2_GetComponentLocation` _crosshair)) (.z (`SceneComponent.K2_GetComponentLocation` _crosshair))) false false))
  (if (> (.y (`SceneComponent.K2_GetComponentLocation` _crosshair_3)) _y)
    (`SceneComponent.K2_SetWorldLocation` _crosshair_3 (`KismetMathLibrary.MakeVector` (.x (`SceneComponent.K2_GetComponentLocation` _crosshair_3)) _y (.z (`SceneComponent.K2_GetComponentLocation` _crosshair_3))) false false)))

(fn `ProcessMove`
  (bind _returnvalue (`GameplayStatics.GetWorldDeltaSeconds`))
  (bind _movespeed (`self.MoveSpeed`))
  (bind _movespeed_2 (`self.MoveSpeed`))
  (bind _absspeedmax (`self.AbsSpeedMax`))
  (bind _returnvalue_2 (* -1.0 _absspeedmax))
  (bind _cube (`/Game/Blueprints/Player.Cube` (`self.mPlayer`)))
  (bind _moveaxis (`self.GetMoveAxis`))
  (if (== _moveaxis 0.0)
    (if (> (`self.MoveSpeed`) 0.0)
      (set `self.MoveSpeed` (+ (`self.MoveSpeed`) (* (* -0.5 (`self.AbsAccel`)) _returnvalue)))
      (if (< (`self.MoveSpeed`) 0.0)
        (set `self.MoveSpeed` 0.0))
      (bind _sweephitresult (`SceneComponent.K2_AddWorldOffset` _cube (`KismetMathLibrary.MakeVector` _movespeed_2) true false :!label _label))
      (if (`GameplayStatics.BreakHitResult` _sweephitresult)
        (`SceneComponent.K2_AddWorldOffset` _cube (`KismetMathLibrary.MakeVector` (* -1.0 _movespeed_2)) false false)
        (set `self.MoveSpeed` 0.0))
      (elif (< (`self.MoveSpeed`) 0.0)
        (set `self.MoveSpeed` (+ (`self.MoveSpeed`) (* (* 0.5 (`self.AbsAccel`)) _returnvalue)))
        (if (> (`self.MoveSpeed`) 0.0)
          (set `self.MoveSpeed` 0.0)
          (goto _label)
          (else
            (goto _label)))))
    (else
      (set `self.MoveSpeed` (+ (`self.MoveSpeed`) (* (* _moveaxis (`self.AbsAccel`)) _returnvalue)))
      (if (<= _movespeed _returnvalue_2)
        (set `self.MoveSpeed` _returnvalue_2)
        (goto _label)
        (elif (>= _movespeed _absspeedmax)
          (set `self.MoveSpeed` _absspeedmax)
          (goto _label)
          (else
            (goto _label)))))))

(fn `SetPawnTransform`
  (params (InTransform :type "Transform Structure"))
  (`self.K2_SetActorTransform` (`self.mPlayer`) InTransform false true))

(fn `UserConstructionScript`)