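; Puck actor that slides and bounces off blocking surfaces, starting with a fixed velocity along negative Y.
; Tick moves the cylinder with a swept offset, applies slight per-frame damping and spins the mesh in proportion to speed.
; Axis-aligned hit normals flip the matching velocity component, other normals reverse both X and Y, and every bounce sheds speed.
; An AngleBetweenVectors helper is defined but not called here.
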(event `self.ReceiveBeginPlay`
  (set `self.mVelocity` (0.0 -500.0 0.0)))

(event `self.ReceiveTick`
  (params (DeltaSeconds :type "Float (single-precision)"))
  (bind _x (.x (`self.mVelocity`)))
  (bind _y (.y (`self.mVelocity`)))
  (bind _z (.z (`self.mVelocity`)))
  (bind _returnvalue (* _x -1.0))
  (bind _returnvalue_2 (* _y -1.0))
  (`SceneComponent.K2_AddRelativeRotation` (`self.PuckMesh`) (`KismetMathLibrary.MakeRotator` 0.0 0.0 (* DeltaSeconds (`KismetMathLibrary.VSize` (`self.mVelocity`)) 0.2)) false false)
  (set `self.mVelocity` (* (`self.mVelocity`) 0.999999))
  (bind _sweephitresult (`SceneComponent.K2_AddWorldOffset` (`self.PuckCylinder`) (* (`self.mVelocity`) DeltaSeconds) true false))
  (bind (_bblockinghit _binitialoverlap _time _location _impactpoint _normal) (`GameplayStatics.BreakHitResult` _sweephitresult))
  (if _bblockinghit
    (if (== (.x _normal) 0.0)
      (set `self.mVelocity` (`KismetMathLibrary.MakeVector` _x _returnvalue_2 _z))
      (elif (== (.y _normal) 0.0)
        (set `self.mVelocity` (`KismetMathLibrary.MakeVector` _returnvalue _y _z))
        (else
          (set `self.mVelocity` (`KismetMathLibrary.MakeVector` _returnvalue _returnvalue_2 _z)))))
    (set `self.mVelocity` (* (`self.mVelocity`) 0.6))))

(fn `AngleBetweenVectors`
  (params (A :type "Vector Structure") (B :type "Vector Structure"))
  (returns (Angle :type "Float (double-precision)"))
  (bind _returnvalue (`KismetMathLibrary.DegAcos` (`KismetMathLibrary.Dot_VectorVector` A B)))
  (if (< (.x A) (.x B))
    (return (- 360.0 _returnvalue))
    (else
      (return _returnvalue))))

(fn `UserConstructionScript`)